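; Player controller for the LMA game that opens the pause, death and end-of-level screens.
; The Pause input, DeadCharacterEvent and EndOfLevelEvent each call a matching widget function.
; Each function, if its stored widget is not valid, pauses the game, creates and shows the widget, switches to UI-only input and shows the cursor.
; Nothing here unpauses the game or clears the widget references.
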(event Custom|EndOfLevelEvent
  (CallFunction|WidgetEndOfLevel))

(event Custom|DeadCharacterEvent
  (CallFunction|WidgetYouAreDead))

(event EventBeginPlay)

(event EventTick
  (params (DeltaSeconds :type Float%20%28single-precision%29)))

(event Input|ActionEvents|InputActionPause
  (params (Key :type Key%20Structure :default "None"))
  (:Pressed
    (CallFunction|WidgetPause)))

(fn ConstructionScript)

(fn WidgetEndOfLevel
  (Variables|Default|GetEndOfLevelWidget
    (:then)
    (:else
      (Game|SetGamePaused true)
      (bind _returnvalue (UserInterface|CreateWidget "/Game/LMA/Widgets/WBP_EndOfLevel.WBP_EndOfLevel_C"))
      (bind _output_get (Variables|Default|SetEndOfLevelWidget _returnvalue))
      (UserInterface|Viewport|AddtoViewport _output_get 0)
      (Input|SetInputModeUIOnly self _output_get "DoNotLock" false)
      (Variables|Default|SetbShowMouseCursor true))))

(fn WidgetYouAreDead
  (Variables|Default|GetYouAreDeadWidget
    (:then)
    (:else
      (Game|SetGamePaused true)
      (bind _returnvalue (UserInterface|CreateWidget "/Game/LMA/Widgets/WBP_YouAreDead.WBP_YouAreDead_C"))
      (bind _output_get (Variables|Default|SetYouAreDeadWidget _returnvalue))
      (UserInterface|Viewport|AddtoViewport _output_get 0)
      (Input|SetInputModeUIOnly self _output_get "DoNotLock" false)
      (Variables|Default|SetbShowMouseCursor true))))

(fn WidgetPause
  (Variables|Default|GetPauseWidget
    (:then)
    (:else
      (Game|SetGamePaused true)
      (bind _returnvalue (UserInterface|CreateWidget "/Game/LMA/Widgets/WBP_Pause.WBP_Pause_C"))
      (bind _output_get (Variables|Default|SetPauseWidget _returnvalue))
      (UserInterface|Viewport|AddtoViewport _output_get 0)
      (Input|SetInputModeUIOnly self _output_get "DoNotLock" false)
      (Variables|Default|SetbShowMouseCursor true))))